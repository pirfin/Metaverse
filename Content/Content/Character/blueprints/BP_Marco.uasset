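; BP_Marco is a player-controlled character that moves and turns through Enhanced Input.
; On possession by a PlayerController it adds the IM_marco mapping context.
; ForwardBackwards and Sides actions add movement along the forward and right vectors of the control rotation's yaw only, ignoring pitch and roll.
; The Turn action adds controller yaw, with no vertical look handled in this graph.
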(event `self.ReceivePossessed`
  (params (NewController :type "Controller Object Reference"))
  (bind _asplayer_controller (cast `PlayerController` NewController))
  (`EnhancedInputSubsystemInterface.AddMappingContext` (pcsubsystem `EnhancedInputLocalPlayerSubsystem` _asplayer_controller) "/Game/Content/Character/Inputs/IM_marco.IM_marco" 0 (struct)))

(event `EnhancedInput|/Game/Content/Character/Inputs/ForwardBackwards`
  (params (ActionValue :type "Float (double-precision)") (ElapsedSeconds :type "Float (double-precision)") (TriggeredSeconds :type "Float (double-precision)") (InputAction :type "InputAction Object Reference" :default "/Game/Content/Character/Inputs/ForwardBackwards.ForwardBackwards"))
  (:`Triggered`
    (`self.AddMovementInput` (`KismetMathLibrary.GetForwardVector` (`KismetMathLibrary.MakeRotator` 0.0 0.0 (.yaw (`self.GetControlRotation`)))) ActionValue)))

(event `EnhancedInput|/Game/Content/Character/Inputs/Sides`
  (params (ActionValue :type "Float (double-precision)") (ElapsedSeconds :type "Float (double-precision)") (TriggeredSeconds :type "Float (double-precision)") (InputAction :type "InputAction Object Reference" :default "/Game/Content/Character/Inputs/Sides.Sides"))
  (:`Triggered`
    (`self.AddMovementInput` (`KismetMathLibrary.GetRightVector` (`KismetMathLibrary.MakeRotator` 0.0 0.0 (.yaw (`self.GetControlRotation`)))) ActionValue)))

(event `EnhancedInput|/Game/Content/Character/Inputs/Turn`
  (params (ActionValue :type "Float (double-precision)") (ElapsedSeconds :type "Float (double-precision)") (TriggeredSeconds :type "Float (double-precision)") (InputAction :type "InputAction Object Reference" :default "/Game/Content/Character/Inputs/Turn.Turn"))
  (:`Triggered`
    (`self.AddControllerYawInput` ActionValue)))

(fn `UserConstructionScript`)